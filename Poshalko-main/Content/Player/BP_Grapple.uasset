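; BP_Grapple defines a paired, one-second grapple finisher against a melee enemy, pairing a toilet leak animation with the victim's death animation at a fixed forward offset.
; On initiation it queues two timed events on the second participant, cast to BP_Enemy_Melee.
; The early event kills the enemy and silences its sound.
; The late event swaps its mesh to the ABP_Sdoh animation blueprint.
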(event `self.On Initiate`
  (`self.Add Queued Event` "Leak" 0.1)
  (`self.Add Queued Event` "ChangeABP" 0.9))

(event `Leak`
  (bind _participant_grapple_component (`/Game/GrappleComponent/BP_GrappleComponent/Utility/ML_GC_GrappleObject.Get Participant by Index (Validated)` 1)
    (:`Is Valid`
      (bind _asbp_enemy_melee (cast `/Game/Enemies/MeleeEnemy/BP_Enemy_Melee` (`ActorComponent.GetOwner` _participant_grapple_component)))
      (`/Game/Enemies/BP_Enemy_Base.Die` _asbp_enemy_melee)
      (`AudioComponent.SetVolumeMultiplier` (`/Game/Enemies/MeleeEnemy/BP_Enemy_Melee.SkibidiCalm` _asbp_enemy_melee) 0.0)
      (`/Game/Enemies/MeleeEnemy/BP_Enemy_Melee.Flush_Sound` _asbp_enemy_melee))))

(event `ChangeABP`
  (bind _participant_grapple_component (`/Game/GrappleComponent/BP_GrappleComponent/Utility/ML_GC_GrappleObject.Get Participant by Index (Validated)` 1)
    (:`Is Valid`
      (bind _asbp_enemy_melee (cast `/Game/Enemies/MeleeEnemy/BP_Enemy_Melee` (`ActorComponent.GetOwner` _participant_grapple_component)))
      (`SkeletalMeshComponent.SetAnimInstanceClass` (`Character.Mesh` _asbp_enemy_melee) "/Game/Characters/Toilets/Toilet1/ABP_Sdoh.ABP_Sdoh_C"))))

(fn `Generate Global Grapple Data`
  (returns (`Global Grapple Data` :type "/Game/GrappleComponent/BP_GrappleComponent/Struct/Struct_GC_GrappleData_Global Structure"))
  (return (`/Game/GrappleComponent/BP_GrappleComponent/Utility/ML_GC_Object.Generate Global Grapple Data (Simplified)` 1.0 "/Game/Characters/Mannequins/Meshes/AS_Leak_Toilet_Small.AS_Leak_Toilet_Small" "/Game/Characters/Toilets/Toilet1/Animations/Male_09Toilet_LeakedDeath.Male_09Toilet_LeakedDeath" (120.0 0.0 0.0) 0.0)))