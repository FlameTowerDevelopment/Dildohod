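; Base pickable item that moves itself into the interacting actor's inventory when Interact fires, then destroys itself.
; It fetches the inventory array through message calls, searches for a slot matching its own class, and writes the updated array back.
; A match stacks CountItems onto that slot, otherwise a new slot is added, each with a debug print.
; Its own GetInventory and SetInventory functions are empty stubs.
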(event `/Game/Systems/InventorySystem/BPI_Interaction.Interact`
  (params (ActorInteract :type "Actor Object Reference"))
  (set `self.Flag` false)
  (bind _inventory (message `/Game/Systems/InventorySystem/BPI_Interaction.GetInventory` ActorInteract))
  (bind _output_get (set `self.OtherInv` _inventory))
  (for (_array_element _array_index) _output_get :!label _label
    (if (== (`.Items_13_21B340124CB82F06045FBE8553D6FDCA` (break `/Game/Systems/InventorySystem/S_Inventory` _array_element)) (`GameplayStatics.GetObjectClass` self))
      (`self.Break`)
      (set `self.Flag` true)
      (set `self.Index` _array_index)))
  (if (`self.Flag`)
    (`self.AddItemCount`
      (:`Next`
        _))
    (else
      (`self.AddItem`
        (:`Next`
          _))))
  (message `/Game/Systems/InventorySystem/BPI_Interaction.SetInventory` ActorInteract (`self.OtherInv`))
  (`self.K2_DestroyActor`))

(event `Break`
  (goto _label :!via `Break`))

(fn `GetInventory`
  (returns (Inventory :type "Array of /Game/Systems/InventorySystem/S_Inventory Structure"))
  (return))

(fn `SetInventory`
  (params (Inventory :type "Array of /Game/Systems/InventorySystem/S_Inventory Structure (by ref)"))
  (returns (`New Inventory` :type "Array of /Game/Systems/InventorySystem/S_Inventory Structure"))
  (return))

(fn `UserConstructionScript`)