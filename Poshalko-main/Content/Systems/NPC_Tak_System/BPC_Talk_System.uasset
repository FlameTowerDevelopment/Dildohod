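; Blueprint component for the NPC talk system that relays messages through an OnMessageAssigned event.
; SendMessage passes a message structure straight to that event.
; A separate CanBeDamaged check, unrelated to talking, routes to do damage, block damage or no damage from the dead, invincible and blocking states, with inputs to override invincibility or allow blocking.
; BeginPlay and Tick are unused.
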(fn `SendMessage`
  (params (MessageStructure :type "/Game/Systems/NPC_Tak_System/S_Talk_System Structure"))
  (`self.OnMessageAssigned` MessageStructure))