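; Player-controlled spider character driven by Enhanced Input, adding its mapping context on BeginPlay for look, move and jump.
; Movement follows control yaw on the horizontal plane, snaps the actor to that yaw and records the last movement time.
; Look input applies only while global time dilation is near normal.
; Camera functions supply a speed-widened FOV, a behind-and-above offset and an unrotated pivot at the actor's location.
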(event `self.ReceiveBeginPlay`
  ;[1 1 1] Setup Input
  (bind _asplayer_controller (cast `PlayerController` (`self.GetController`)))
  (bind _output_get (set `self.PlayerController` _asplayer_controller))
  (bind _returnvalue (pcsubsystem `EnhancedInputLocalPlayerSubsystem` _output_get))
  (`/Engine/EditorBlueprintResources/StandardMacros.IsValid` _returnvalue
    (:`Is Valid`
      (`EnhancedInputSubsystemInterface.AddMappingContext` _returnvalue "/Game/Input/IMC_Spider.IMC_Spider" 0 (struct)))))

(event `EnhancedInput|/Game/Input/Actions/IA_Look`
  (params (ActionValue :type "Vector2D Structure") (ElapsedSeconds :type "Float (double-precision)") (TriggeredSeconds :type "Float (double-precision)") (InputAction :type "InputAction Object Reference" :default "/Game/Input/Actions/IA_Look.IA_Look"))
  (:`Triggered`
    ;[1 1 1] Handle Look
    (if (`KismetMathLibrary.NearlyEqual_FloatFloat` (`GameplayStatics.GetGlobalTimeDilation`) 1.0 0.01)
      (`|ExecutionSequence`
        (:`then_0`
          (`self.AddControllerPitchInput` ActionValue_Y))
        (:`then_1`
          (`self.AddControllerYawInput` ActionValue_X))))))

(event `EnhancedInput|/Game/Input/Actions/IA_Move`
  (params (ActionValue :type "Vector2D Structure") (ElapsedSeconds :type "Float (double-precision)") (TriggeredSeconds :type "Float (double-precision)") (InputAction :type "InputAction Object Reference" :default "/Game/Input/Actions/IA_Move.IA_Move"))
  (bind (_returnvalue_roll _returnvalue_pitch _returnvalue_yaw) (`KismetMathLibrary.BreakRotator` (`self.GetControlRotation`)))
  (bind (_returnvalue_roll_2 _returnvalue_pitch_2 _returnvalue_yaw_2) (`KismetMathLibrary.BreakRotator` (`self.GetControlRotation`)))
  (bind (_returnvalue_roll_3 _returnvalue_pitch_3 _returnvalue_yaw_3) (`KismetMathLibrary.BreakRotator` (`self.GetControlRotation`)))
  (bind (_returnvalue_x _returnvalue_y) (`KismetMathLibrary.BreakVector` (+ (* ActionValue_X (`KismetMathLibrary.GetRightVector` (`KismetMathLibrary.MakeRotator` _returnvalue_roll_2 0.0 _returnvalue_yaw_2))) (* ActionValue_Y (`KismetMathLibrary.GetForwardVector` (`KismetMathLibrary.MakeRotator` 0.0 0.0 _returnvalue_yaw))))))
  (:`Triggered`
    ;[1 1 1] Handle Move
    (`self.AddMovementInput` (`KismetMathLibrary.Normal` (`KismetMathLibrary.MakeVector` _returnvalue_x _returnvalue_y) 0.01))
    (set `self.LastMovementFrame` (`GameplayStatics.GetTimeSeconds`))
    (`self.K2_SetActorRotation` (`KismetMathLibrary.MakeRotator` 0.0 0.0 _returnvalue_yaw_3))))

(event `EnhancedInput|/Game/Input/Actions/IA_Jump`
  (params (ActionValue :type Boolean) (ElapsedSeconds :type "Float (double-precision)") (TriggeredSeconds :type "Float (double-precision)") (InputAction :type "InputAction Object Reference" :default "/Game/Input/Actions/IA_Jump.IA_Jump"))
  (:`Triggered`
    ;[1 1 1] HandleJump
    (`self.Jump`))
  (:`Completed`
    (`self.StopJumping`)))

(event `self.ReceiveTick`
  (params (DeltaSeconds :type "Float (single-precision)")))

(fn `GetCameraParameters`
  (returns (FOV :type "Float (double-precision)") (Offset :type "Vector Structure"))
  (return (+ (* (/ (`KismetMathLibrary.VSizeXY` (`self.GetVelocity`)) (`MovementComponent.GetMaxSpeed` (`self.CharacterMovement`))) 10.0) 80.0) (-200.0 0.0 30.0)))

(fn `GetViewSocket`
  (returns (Socket :type "Transform Structure"))
  (return (`KismetMathLibrary.MakeTransform` (`self.K2_GetActorLocation`))))

(fn `UserConstructionScript`)