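; BP_FireGun is a flamethrower weapon that damages actors in front of the player's camera while firing.
; Fire starts the flame particles, looping damage logic, audio and a camera shake on the player.
; Every 0.2 seconds a short camera-forward line trace, with debug drawing enabled, damages any hit actor's BP_HealthComponent.
; UnFire clears the IsFire flag to end the loop and stops the effects.
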(event `Fire`
  (bind _returnvalue (`GameplayStatics.GetPlayerCameraManager` 0))
  (bind _returnvalue_2 (`PlayerCameraManager.GetCameraLocation` _returnvalue))
  (bind _returnvalue_3 (`self.GetComponentByClass` (`GameplayStatics.GetPlayerCharacter` 0) "/Script/Engine.CameraShakeSourceComponent"))
  (set `self.IsFire` true)
  (`ActorComponent.Activate` (`self.P_FlameThrower2_Converted`) false)
  (`AudioComponent.Play` (`self.Audio`) 0.0)
  (`/Engine/EditorBlueprintResources/StandardMacros.IsValid` _returnvalue_3
    (:`Is Valid`
      (`CameraShakeSourceComponent.StartCameraShake` :`self` _returnvalue_3 :`InCameraShake` "/Game/Characters/Cameraman/BP/BP_CameraShakeFiregun.BP_CameraShakeFiregun_C"))
    (:`Is Not Valid`
      _))
  (bind (_outhit _returnvalue_4) (`KismetSystemLibrary.LineTraceSingle` _returnvalue_2 (+ _returnvalue_2 (* (`KismetMathLibrary.GetForwardVector` (`PlayerCameraManager.GetCameraRotation` _returnvalue)) 600.0)) "TraceTypeQuery1" false (`|MakeArray` (`GameplayStatics.GetPlayerCharacter` 0) :!type "Actor Object Reference") "ForDuration" :!label _label))
  (if _returnvalue_4
    (bind _returnvalue_5 (`self.GetComponentByClass` (`.HitActor` (`GameplayStatics.BreakHitResult` _outhit)) "/Game/Characters/BP_HealthComponent.BP_HealthComponent_C"))
    (`/Engine/EditorBlueprintResources/StandardMacros.IsValid` _returnvalue_5
      (:`Is Valid`
        (`/Game/Characters/BP_HealthComponent.TakeDamage` _returnvalue_5 0.5))
      (:`Is Not Valid`
        _)))
  (`KismetSystemLibrary.Delay` 0.2)
  (if (`self.IsFire`)
    (goto _label)))

(event `UnFire`
  (set `self.IsFire` false)
  (`AudioComponent.Stop` (`self.Audio`))
  (`ActorComponent.Deactivate` (`self.P_FlameThrower2_Converted`))
  (`CameraShakeSourceComponent.StopAllCameraShakesOfType` (`self.GetComponentByClass` (`GameplayStatics.GetPlayerCharacter` 0) "/Script/Engine.CameraShakeSourceComponent") "/Game/Characters/Cameraman/BP/BP_CameraShakeFiregun.BP_CameraShakeFiregun_C" true))

(fn `UserConstructionScript`)