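; BP_DartGun is the cameraman character's dart gun, which shoots BP_Dart projectiles when its Fire event is called.
; Fire plays the shoot montage on the player mesh, plays a gunshot sound and spawns a dart at the gun's Scene component, aimed along the camera rotation.
; It then adds pitch and random yaw recoil to the player, while a DoOnce reset after a short delay limits the fire rate.
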(event `Fire`
  (bind _returnvalue (`GameplayStatics.GetPlayerCharacter` 0))
  (`/Engine/EditorBlueprintResources/StandardMacros.DoOnce` false :!label _label
    (:`Completed`
      (`|ExecutionSequence`
        (:`then_0`
          (`|PlayMontage` (`Character.Mesh` (`GameplayStatics.GetPlayerCharacter` 0)) "/Game/Characters/Cameraman/Animations/DartGun/AS_Cameraman_DartGunShoot_Montage.AS_Cameraman_DartGunShoot_Montage"
            (:`then`
              (`GameplayStatics.PlaySoundAtLocation` "/Game/Characters/TitanCameramen2_0/Sounds/SW_ShoulderGunShoot.SW_ShoulderGunShoot" (`self.K2_GetActorLocation`) (struct) 1.0 1.0 0.0 null null null null)
              (`|SpawnActorFromClass` "/Game/Characters/Cameraman/Ammunitions/DartGun/BP/BP_Dart.BP_Dart_C" (`KismetMathLibrary.MakeTransform` (`SceneComponent.K2_GetComponentLocation` (`self.Scene`)) (`PlayerCameraManager.GetCameraRotation` (`GameplayStatics.GetPlayerCameraManager` 0))) "Undefined" "MultiplyWithRoot" null null)
              (`Pawn.AddControllerPitchInput` _returnvalue -2.0)
              (`Pawn.AddControllerYawInput` _returnvalue (`KismetMathLibrary.RandomFloatInRange` -1.5 1.5)))))
        (:`then_1`
          (`KismetSystemLibrary.Delay` 0.4)
          (goto _label :!via `Reset`))))))

(fn `UserConstructionScript`)