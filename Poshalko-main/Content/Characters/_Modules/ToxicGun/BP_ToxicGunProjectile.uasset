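; BP_ToxicGunProjectile is the toxic gun's projectile, exploding on contact to deal direct and area damage through BP_HealthComponent.
; Capsule overlap events switch on shortly after spawn, and both overlap and hit events share one impact path.
; It damages the overlapped actor, then nearby pawns except player 0, so a directly struck pawn can take damage twice.
; The projectile then destroys itself and spawns an explosion effect.
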(event `self.ReceiveBeginPlay`
  (`KismetSystemLibrary.Delay` 0.1)
  (set `PrimitiveComponent.bGenerateOverlapEvents` true (`self.Capsule`)))

(event `self.Capsule.OnComponentBeginOverlap`
  (params (OverlappedComponent :type "PrimitiveComponent Object Reference") (OtherActor :type "Actor Object Reference") (OtherComp :type "PrimitiveComponent Object Reference") (OtherBodyIndex :type Integer) (bFromSweep :type Boolean) (SweepResult :type "HitResult Structure (by ref)"))
  (bind _returnvalue (`self.GetComponentByClass` OtherActor "/Game/Characters/BP_HealthComponent.BP_HealthComponent_C"))
  (`|ExecutionSequence` :!label _label
    (:`then_0`
      (`/Engine/EditorBlueprintResources/StandardMacros.IsValid` _returnvalue
        (:`Is Valid`
          (`/Game/Characters/BP_HealthComponent.TakeDamage` _returnvalue 3.0))
        (:`Is Not Valid`
          _))
      (bind _outactors (`KismetSystemLibrary.SphereOverlapActors` (`self.K2_GetActorLocation`) 100.0 (`|MakeArray` "ObjectTypeQuery3" :!type "EObjectTypeQuery Enum")))
      (`KismetArrayLibrary.Array_RemoveItem` _outactors (`GameplayStatics.GetPlayerCharacter` 0))
      (for _array_element _outactors
        (bind _returnvalue_2 (`self.GetComponentByClass` _array_element "/Game/Characters/BP_HealthComponent.BP_HealthComponent_C"))
        (`/Engine/EditorBlueprintResources/StandardMacros.IsValid` _returnvalue_2
          (:`Is Valid`
            (`/Game/Characters/BP_HealthComponent.TakeDamage` _returnvalue_2 3.0))))
      (`self.K2_DestroyActor`))
    (:`then_1`
      (`GameplayStatics.SpawnEmitterAtLocation` "/Game/VFX/Realistic_Starter_VFX_Pack_Vol2/Particles/Explosion/P_Explosion_Big_A.P_Explosion_Big_A" (`self.K2_GetActorLocation`) (struct) (2.0 2.0 2.0)))))

(event `self.Capsule.OnComponentHit`
  (params (HitComponent :type "PrimitiveComponent Object Reference") (OtherActor :type "Actor Object Reference") (OtherComp :type "PrimitiveComponent Object Reference") (NormalImpulse :type "Vector Structure") (Hit :type "HitResult Structure (by ref)"))
  (goto _label))

(fn `UserConstructionScript`)