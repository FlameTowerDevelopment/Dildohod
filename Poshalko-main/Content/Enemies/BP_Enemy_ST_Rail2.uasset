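; BP_Enemy_ST_Rail2 is an enemy Blueprint that, as it stands, is a skeleton with no behavior of its own.
; BeginPlay, Tick and construction defer to the parent, and Tick's AttackTarget validity check leads nowhere.
; The attack, health, healing and range functions are stubs returning false or zero.
; An unwired MediumLaser reference and look-at rotation toward AttackTarget remain in the event graph.
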(event `self.ReceiveBeginPlay`
  (`parent.ReceiveBeginPlay`))

(event `self.ReceiveTick`
  (params (DeltaSeconds :type "Float (single-precision)"))
  (`parent.ReceiveTick` DeltaSeconds)
  (`/Engine/EditorBlueprintResources/StandardMacros.IsValid` (`self.AttackTarget`)))

(fn `AttackStart`
  (params (AttackTarget :type "Actor Object Reference") (TokensNeeded :type Integer))
  (returns (Success :type Boolean))
  (return false))

(fn `GetCurrentHealth`
  (returns (Health :type "Float (double-precision)"))
  (return 0.0))

(fn `GetIdealRange`
  (returns (AttackRadius :type "Float (double-precision)") (DefendRadius :type "Float (double-precision)"))
  (return 0.0 0.0))

(fn `Heal`
  (params (Amount :type "Float (double-precision)"))
  (returns (NewHealth :type "Float (double-precision)"))
  (return 0.0))

(fn `IsAttacking`
  (returns (Attacking :type Boolean))
  (return false))

(fn `UserConstructionScript`
  (`parent.UserConstructionScript`))