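; Plunger boss enemy character that provides melee attacks, sword equipping and dodges, plus movement speed and combat range settings.
; Ground smash, short-range, long-range and spinning attacks pass attack info to BPCAttacks, with randomized montages for long range.
; Montage notifies spawn and attach or destroy the sword, and completion fires equip or unequip callbacks.
; Projectile and melee dodges play random montages with invincibility, cleared on completion or interruption.
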(event `GroundSmashAttack`
  (params (AttackTarget :type "Actor Object Reference"))
  ;[1 1 1] Attacks
  (`/Game/Systems/Attacks/BPC_Attacks.GroundSmash` (`self.BPC_Attacks`) (make `/Game/Systems/Attacks/S_AttackInfo` AttackTarget "/Game/Animations/Melee/Montage_Melee_GroundSmash.Montage_Melee_GroundSmash" (make `/Game/Systems/DamageSystem/S_DamageInfo` 25.0 "NewEnumerator0" "NewEnumerator3")) 300.0))

(event `ShortRangeAttack`
  (params (AttackTarget :type "Actor Object Reference"))
  (bind (_outitem _outindex) (`KismetArrayLibrary.Array_Random` (`|MakeArray` "/Game/FightAnimations/Montages/Combat/AM_Combo_R2.AM_Combo_R2" "/Game/FightAnimations/Montages/Combat/AM_Combo_L2_R1.AM_Combo_L2_R1" "/Game/FightAnimations/Montages/Combat/AM_Combo_R1.AM_Combo_R1" "/Game/FightAnimations/Montages/Combat/AM_Combo_L3.AM_Combo_L3" "/Game/FightAnimations/Montages/Combat/AM_Combo_L2.AM_Combo_L2" :!type "AnimMontage Object Reference")))
  ;[1 1 1] Attacks
  (`/Game/Systems/Attacks/BPC_Attacks.PrimaryMeleeAttack` (`self.BPC_Attacks`) (make `/Game/Systems/Attacks/S_AttackInfo` AttackTarget _outitem (`|GetArrayItem` (`|MakeArray` (make `/Game/Systems/DamageSystem/S_DamageInfo` 25.0 "NewEnumerator2" "NewEnumerator1" "NewEnumerator0" true true true) (make `/Game/Systems/DamageSystem/S_DamageInfo` 40.0 "NewEnumerator1" "NewEnumerator1" "NewEnumerator4" false true true true) (make `/Game/Systems/DamageSystem/S_DamageInfo` 50.0 "NewEnumerator1" "NewEnumerator1" "NewEnumerator1" false true true true) (make `/Game/Systems/DamageSystem/S_DamageInfo` 45.0 "NewEnumerator1" "NewEnumerator1" "NewEnumerator4" true true true true) (make `/Game/Systems/DamageSystem/S_DamageInfo` 35.0 "NewEnumerator2" "NewEnumerator1" "NewEnumerator0" true true true)) _outindex)) 20.0 200.0 (`|GetArrayItem` (`|MakeArray` 55.0 0.0 55.0 0.0 55.0) _outindex)))

(event `LongRangeAttack`
  (params (AttackTarget :type "Actor Object Reference"))
  ;[1 1 1] Attacks
  (`/Game/Systems/Attacks/BPC_Attacks.LongRangeMeleeAttack` (`self.BPC_Attacks`) (make `/Game/Systems/Attacks/S_AttackInfo` AttackTarget (`KismetArrayLibrary.Array_Random` (`|MakeArray` "/Game/FightAnimations/Montages/Combat/AM_Combo_R1_L1.AM_Combo_R1_L1" "/Game/FightAnimations/Montages/Combat/AM_Combo_R1.AM_Combo_R1" :!type "AnimMontage Object Reference")) (make `/Game/Systems/DamageSystem/S_DamageInfo` 25.0 "NewEnumerator0" "NewEnumerator1" "NewEnumerator0" false true true))))

(event `SpinningAttack`
  (params (AttackTarget :type "Actor Object Reference"))
  ;[1 1 1] Attacks
  (`/Game/Systems/Attacks/BPC_Attacks.SpinningMeleeAttack` (`self.BPC_Attacks`) (make `/Game/Systems/Attacks/S_AttackInfo` AttackTarget "/Game/Animations/Melee/Montage_Sword_SpinningAttack.Montage_Sword_SpinningAttack" (make `/Game/Systems/DamageSystem/S_DamageInfo` 10.0 "NewEnumerator0" "NewEnumerator1" "NewEnumerator0" false true))))

(event `/Game/Enemies/AI/BPI_EnemyAI.EquipWeapon`
  ;[1 1 1] Equip/Unequip weapon
  (bind _notifyname (`|PlayMontage` (`self.Mesh`) "/Game/FightAnimations/Montages/AM_Taunt_UE_Montage.AM_Taunt_UE_Montage")
    (:`OnCompleted`
      (`self.OnWeaponEquipped`))
    (:`OnNotifyBegin`
      (switch `name` _notifyname
        (:`HoldSword`
          (bind _returnvalue (`|SpawnActorFromClass` "/Game/Weapons/BP_Weapon_Sword.BP_Weapon_Sword_C" (`self.GetTransform`) "Undefined" "MultiplyWithRoot" null null))
          (bind _output_get (set `self.WeaponActor` _returnvalue))
          (`self.K2_AttachToComponent` _output_get (`self.Mesh`) "hand_r_sword_socket" "SnapToTarget" "SnapToTarget" "SnapToTarget" true)
          (set `self.IsWieldingWeapon` true))))))

(event `/Game/Enemies/AI/BPI_EnemyAI.UnequipWeapon`
  ;[1 1 1] Equip/Unequip weapon
  (bind _notifyname (`|PlayMontage` (`self.Mesh`) "/Game/FightAnimations/Montages/AM_Loser_UE_Montage.AM_Loser_UE_Montage")
    (:`OnCompleted`
      (`self.OnWeaponUnequipped`))
    (:`OnNotifyBegin`
      (switch `name` _notifyname
        (:`DropSword`
          (`self.K2_DestroyActor` (`self.WeaponActor`))
          (set `self.IsWieldingWeapon` false))))))

(event `/Game/Enemies/AI/BPI_EnemyAI.DodgeProjectiles`
  ;[1 1 1] Equip/Unequip weapon
  (set `/Game/Systems/DamageSystem/BPC_DamageSystem.IsInvincible` true (`self.BPC_DamageSystem`))
  (`|PlayMontage` (`self.Mesh`) (select `int` (`KismetMathLibrary.RandomInteger` 2) :`0` "/Game/Animations/WeaponAnimations/Dodge/NewDodge/RollLeft_Root_Montage.RollLeft_Root_Montage" :`1` "/Game/Animations/WeaponAnimations/Dodge/NewDodge/RollRight_Root_Montage.RollRight_Root_Montage" :`2` "/Game/Animations/WeaponAnimations/Dodge/NewDodge/RollBackward_Root_Montage.RollBackward_Root_Montage" :!type "AnimMontage Object Reference")
    (:`OnCompleted`
      _)
    (:`OnInterrupted`
      _))
  (`self.OnDodged`)
  (set `/Game/Systems/DamageSystem/BPC_DamageSystem.IsInvincible` false (`self.BPC_DamageSystem`)))

(event `/Game/Enemies/AI/BPI_EnemyAI.DodgeMelle`
  ;[1 1 1] Equip/Unequip weapon
  (set `/Game/Systems/DamageSystem/BPC_DamageSystem.IsInvincible` true (`self.BPC_DamageSystem`))
  (`|PlayMontage` (`self.Mesh`) (select `int` (`KismetMathLibrary.RandomInteger` 2) :`0` "/Game/FightAnimations/Montages/Dodges/A_Dodge_L1_Montage.A_Dodge_L1_Montage" :`1` "/Game/FightAnimations/Montages/Dodges/A_Dodge_R1_Montage.A_Dodge_R1_Montage" :`2` "/Game/FightAnimations/Montages/Dodges/A_Dodge_B1_Montage.A_Dodge_B1_Montage" :!type "AnimMontage Object Reference")
    (:`OnCompleted`
      _)
    (:`OnInterrupted`
      _))
  (`self.OnDodged`)
  (set `/Game/Systems/DamageSystem/BPC_DamageSystem.IsInvincible` false (`self.BPC_DamageSystem`)))

(fn `GetIdealRange`
  (returns (AttackRadius :type "Float (double-precision)") (DefendRadius :type "Float (double-precision)"))
  (return 600.0 1488.0))

(fn `SetMovementSpeed`
  (params (Speed :type "/Game/Enemies/AI/Enums/E_MovementSpeed Enum" :default "NewEnumerator0"))
  (returns (SpeedValue :type "Float (double-precision)"))
  (bind _output_get (set `CharacterMovementComponent.MaxWalkSpeed` (select `/Game/Enemies/AI/Enums/E_MovementSpeed` Speed :`NewEnumerator1` 100.0 :`NewEnumerator2` 300.0 :`NewEnumerator3` 500.0 :!type "Float (single-precision)") (`self.CharacterMovement`)))
  (return _output_get))

(fn `UserConstructionScript`
  (`parent.UserConstructionScript`))