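; BP_Daun is a character, filed under enemies, that reacts to talk-system messages addressed to it.
; TakeMessage ignores other recipients, otherwise prints the subtitles and snaps the capsule to the full look-at rotation toward the sender.
; After the message's answer time, it plays a waving montage on the mesh.
; BeginPlay binds to BPCTalkSystem's OnMessageAssigned, but that handler is empty.
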(event `self.ReceiveBeginPlay`
  (add `/Game/Systems/NPC_Tak_System/BPC_Talk_System.OnMessageAssigned` (`self.BPC_Talk_System`) (delegate `OnMessageAssigned_Event`)))

(event `OnMessageAssigned_Event`
  (params (Message_Structure :type "/Game/Systems/NPC_Tak_System/S_Talk_System Structure")))

(event `/Game/Systems/NPC_Tak_System/BPI_TalkSystem.TakeMessage`
  (params (MyMessage :type "/Game/Systems/NPC_Tak_System/S_Talk_System Structure"))
  (bind (_sender _recipient _subtitles _needresponce _answertime) (break `/Game/Systems/NPC_Tak_System/S_Talk_System` MyMessage))
  (if (== _recipient self)
    (`KismetSystemLibrary.PrintString` (`KismetTextLibrary.Conv_TextToString` _subtitles))
    (`SceneComponent.K2_SetWorldRotation` (`self.CapsuleComponent`) (`KismetMathLibrary.FindLookAtRotation` (`self.K2_GetActorLocation`) (`self.K2_GetActorLocation` _sender)) false false)
    (`KismetSystemLibrary.Delay` _answertime)
    (`|PlayMontage` (`self.Mesh`) "/Game/Animations/TalkAnim/A_Waving_UE_Montage.A_Waving_UE_Montage")))

(fn `UserConstructionScript`)