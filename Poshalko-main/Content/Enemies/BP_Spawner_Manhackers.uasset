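; Spawner actor that creates flying manhack enemies when it receives a summon message.
; TakeMessage spawns the manhack at the spawner's location, passes the message sender as its attack target, calls its spawn hook and sets its movement to flying.
; A DoOnce gate, reset by a custom event after a short delay, throttles repeat summons.
; Any other message also closes the gate, with no reset on that path.
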(event `/Game/Systems/NPC_Tak_System/BPI_TalkSystem.TakeMessage`
  (params (MyMessage :type "/Game/Systems/NPC_Tak_System/S_Talk_System Structure"))
  (bind (_sender _recipient _subtitles _needresponce _answertime _id) (break `/Game/Systems/NPC_Tak_System/S_Talk_System` MyMessage))
  (bind _returnvalue_location (`KismetMathLibrary.BreakTransform` (`self.GetTransform`)))
  (`/Engine/EditorBlueprintResources/StandardMacros.DoOnce` false :!label _label
    (:`Completed`
      (if (== _id "SUMMON_MANHACK")
        (bind _returnvalue (`|SpawnActorFromClass` "/Game/Enemies/BP_Enemy_ST_Fly_Manhack.BP_Enemy_ST_Fly_Manhack_C" (`KismetMathLibrary.MakeTransform` _returnvalue_location) "Undefined" "MultiplyWithRoot" null 2 _sender null))
        (`/Game/Enemies/BP_Enemy_ST_Fly_Manhack.On spawned` _returnvalue)
        (`CharacterMovementComponent.SetMovementMode` (`Character.CharacterMovement` _returnvalue) "MOVE_Flying" 0)
        (`KismetSystemLibrary.PrintText` "Полетели")
        (`KismetSystemLibrary.Delay` 1.0)
        (`self.Fuck`)))))

(event `Fuck`
  (goto _label :!via `Reset`))

(fn `UserConstructionScript`)