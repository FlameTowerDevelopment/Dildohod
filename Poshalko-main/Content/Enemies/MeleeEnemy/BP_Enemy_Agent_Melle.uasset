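; BP_Enemy_Agent_Melle is a melee enemy agent with ground smash, short-range, long-range jump and spinning attacks.
; Each attack event packs target, montage and damage into an attack info struct for the BPCAttacks component, with some montages picked at random.
; Equip and unequip play taunt and loser montages, using notifies to spawn a hand-socketed sword or destroy it, then signal completion.
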(event `self.ReceiveBeginPlay`
  (`parent.ReceiveBeginPlay`))

(event `self.ReceiveTick`
  (params (DeltaSeconds :type "Float (single-precision)")))

(event `GroundSmashAttack`
  (params (AttackTarget :type "Actor Object Reference"))
  ;[1 1 1] Attacks
  (`/Game/Systems/Attacks/BPC_Attacks.GroundSmash` (`self.BPC_Attacks`) (make `/Game/Systems/Attacks/S_AttackInfo` AttackTarget "/Game/Animations/Melee/Montage_Melee_GroundSmash.Montage_Melee_GroundSmash" (make `/Game/Systems/DamageSystem/S_DamageInfo` 25.0 "NewEnumerator0" "NewEnumerator3")) 300.0))

(event `ShortRangeAttack`
  (params (AttackTarget :type "Actor Object Reference"))
  ;[1 1 1] Attacks
  (`/Game/Systems/Attacks/BPC_Attacks.PrimaryMeleeAttack` (`self.BPC_Attacks`) (make `/Game/Systems/Attacks/S_AttackInfo` AttackTarget (`KismetArrayLibrary.Array_Random` (`|MakeArray` "/Game/FightAnimations/Montages/Combat/AM_HK_Round.AM_HK_Round" "/Game/FightAnimations/Montages/Combat/AM_FrontKick_Havy1_Montage.AM_FrontKick_Havy1_Montage" "/Game/FightAnimations/Montages/Combat/AM_HK_Round.AM_HK_Round" "/Game/FightAnimations/Montages/Combat/AM_OverHand_R1_Montage.AM_OverHand_R1_Montage" "/Game/FightAnimations/Montages/Combat/AM_BackFist_L1_Montage.AM_BackFist_L1_Montage" :!type "AnimMontage Object Reference")) (make `/Game/Systems/DamageSystem/S_DamageInfo` 50.0 "NewEnumerator0" "NewEnumerator1" "NewEnumerator0" false true true)) 20.0 200.0))

(event `LongRangeAttack`
  (params (AttackTarget :type "Actor Object Reference"))
  ;[1 1 1] Attacks
  (`/Game/Systems/Attacks/BPC_Attacks.LongRangeMeleeAttack` (`self.BPC_Attacks`) (make `/Game/Systems/Attacks/S_AttackInfo` AttackTarget (`KismetArrayLibrary.Array_Random` (`|MakeArray` "/Game/FightAnimations/Montages/Combat/AM_Jump_Attack_Fist.AM_Jump_Attack_Fist" "/Game/FightAnimations/Montages/Combat/AM_AxeKick_Jump1_Montage.AM_AxeKick_Jump1_Montage" :!type "AnimMontage Object Reference")) (make `/Game/Systems/DamageSystem/S_DamageInfo` 25.0 "NewEnumerator0" "NewEnumerator1" "NewEnumerator0" false true true))))

(event `SpinningAttack`
  (params (AttackTarget :type "Actor Object Reference"))
  ;[1 1 1] Attacks
  (`/Game/Systems/Attacks/BPC_Attacks.SpinningMeleeAttack` (`self.BPC_Attacks`) (make `/Game/Systems/Attacks/S_AttackInfo` AttackTarget "/Game/Animations/Melee/Montage_Sword_SpinningAttack.Montage_Sword_SpinningAttack" (make `/Game/Systems/DamageSystem/S_DamageInfo` 10.0 "NewEnumerator0" "NewEnumerator1" "NewEnumerator0" false true))))

(event `/Game/Enemies/AI/BPI_EnemyAI.EquipWeapon`
  ;[1 1 1] Equip/Unequip weapon
  (bind _notifyname (`|PlayMontage` (`self.Mesh`) "/Game/FightAnimations/Montages/AM_Taunt_UE_Montage.AM_Taunt_UE_Montage")
    (:`OnCompleted`
      (`self.OnWeaponEquipped`))
    (:`OnNotifyBegin`
      (switch `name` _notifyname
        (:`HoldSword`
          (bind _returnvalue (`|SpawnActorFromClass` "/Game/Weapons/BP_Weapon_Sword.BP_Weapon_Sword_C" (`self.GetTransform`) "Undefined" "MultiplyWithRoot" null null))
          (bind _output_get (set `self.WeaponActor` _returnvalue))
          (`self.K2_AttachToComponent` _output_get (`self.Mesh`) "hand_r_sword_socket" "SnapToTarget" "SnapToTarget" "SnapToTarget" true)
          (set `self.IsWieldingWeapon` true))))))

(event `/Game/Enemies/AI/BPI_EnemyAI.UnequipWeapon`
  ;[1 1 1] Equip/Unequip weapon
  (bind _notifyname (`|PlayMontage` (`self.Mesh`) "/Game/FightAnimations/Montages/AM_Loser_UE_Montage.AM_Loser_UE_Montage")
    (:`OnCompleted`
      (`self.OnWeaponUnequipped`))
    (:`OnNotifyBegin`
      (switch `name` _notifyname
        (:`DropSword`
          (`self.K2_DestroyActor` (`self.WeaponActor`))
          (set `self.IsWieldingWeapon` false))))))

(fn `UserConstructionScript`
  (`parent.UserConstructionScript`))