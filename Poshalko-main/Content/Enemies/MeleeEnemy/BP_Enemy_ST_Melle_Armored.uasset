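; Armored melee enemy Blueprint that pushes its Armor value into the damage system component on BeginPlay.
; Damage and death queries forward to BPCDamageSystem, while attacking and current health queries return fixed stub values.
; Setters drive CharacterMovement speed by movement state, acceleration and velocity, and a toggle switches two particle systems and a rocket sound.
; Tick also prints debug strings every frame.
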(event `self.ReceiveBeginPlay`
  (`parent.ReceiveBeginPlay`)
  (`/Game/Systems/DamageSystem/BPC_DamageSystem.Edit Hitbox Armor` (`self.BPC_DamageSystem`) (`self.Armor`)))

(event `self.ReceiveTick`
  (params (DeltaSeconds :type "Float (single-precision)"))
  (`parent.ReceiveTick` DeltaSeconds)
  (`KismetSystemLibrary.PrintString` "Hello" true true (struct :`G` 0.66 :`B` 1.0 :`A` 1.0) DeltaSeconds)
  (`KismetSystemLibrary.PrintString` "Hello" true true (struct :`G` 0.66 :`B` 1.0 :`A` 1.0) DeltaSeconds))

(event `/Game/Systems/DamageSystem/BPI_Damagable.SetIsInterruptible`
  (params (Value :type Boolean)))

(event `/Game/Enemies/AI/BPI_EnemyAI.SetAccelerator`
  (params (Acceleration :type "Float (double-precision)"))
  (set `CharacterMovementComponent.MaxAcceleration` Acceleration (`self.CharacterMovement`)))

(event `/Game/Enemies/AI/BPI_EnemyAI.SetVelocity`
  (params (Velocity :type "Float (double-precision)"))
  (set `MovementComponent.Velocity` (`KismetMathLibrary.Conv_DoubleToVector` Velocity) (`self.CharacterMovement`)))

(event `/Game/Characters/BPI_Effects.EffectsGroupToogle`
  (params (Enabled :type Boolean))
  (`ActorComponent.SetActive` (`self.ParticleSystem`) Enabled false)
  (`ActorComponent.SetActive` (`self.ParticleSystem1`) Enabled false)
  (`ActorComponent.SetActive` (`self.RocketSound`) Enabled true))

(fn `GetCurrentHealth`
  (returns (Health :type "Float (double-precision)"))
  (return 0.0))

(fn `IsAttacking`
  (returns (Attacking :type Boolean))
  (return false))

(fn `IsDead`
  (returns (Dead :type Boolean))
  (return (`/Game/Systems/DamageSystem/BPC_DamageSystem.IsDead` (`self.BPC_DamageSystem`))))

(fn `SetMovementSpeed`
  (params (Speed :type "/Game/Enemies/AI/Enums/E_MovementSpeed Enum" :default "NewEnumerator0"))
  (returns (SpeedValue :type "Float (double-precision)"))
  (bind _output_get (set `CharacterMovementComponent.MaxWalkSpeed` (select `/Game/Enemies/AI/Enums/E_MovementSpeed` Speed :`NewEnumerator1` 100.0 :`NewEnumerator2` 300.0 :`NewEnumerator3` 600.0 :`NewEnumerator4` 5000.0) (`self.CharacterMovement`)))
  (return _output_get))

(fn `TakeDamage`
  (params (DamageInfo :type "/Game/Systems/DamageSystem/S_DamageInfo Structure") (`Damage Causer` :type "Actor Object Reference") (TagEnter :type Name))
  (returns (WasDamaged :type Boolean))
  (bind _wasdamaged (`/Game/Systems/DamageSystem/BPC_DamageSystem.TakeDamage` (`self.BPC_DamageSystem`) DamageInfo `Damage Causer` "None"))
  (return _wasdamaged))

(fn `UserConstructionScript`
  (`parent.UserConstructionScript`))