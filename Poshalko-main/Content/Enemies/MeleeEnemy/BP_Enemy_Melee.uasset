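; BP_Enemy_Melee is a melee enemy that bites and spins to attack and can draw or sheathe a sword.
; Each attack event passes target, montage and damage info to the BPCAttacks component.
; Montage notifies spawn and socket-attach or destroy the sword, while SkibidiCalm audio mutes, then swaps between calm and attack sounds on completion.
; It also supplies ideal ranges and velocity-based location prediction; TakeDamage and IsDead simply return false.
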(event `self.ReceiveBeginPlay`
  (`parent.ReceiveBeginPlay`))

(event `self.ReceiveTick`
  (params (DeltaSeconds :type "Float (single-precision)")))

(event `GroundSmashAttack`
  (params (AttackTarget :type "Actor Object Reference"))
  ;[1 1 1] Attacks
  (`/Game/Attacks/BPC_Attacks.GroundSmash` (`self.BPC_Attacks`) (make `/Game/Attacks/S_AttackInfo` AttackTarget "/Game/Characters/Toilets/Toilet1/Animations/AM_Bite.AM_Bite" (make `/Game/DamageSystem/S_DamageInfo` 25.0 "NewEnumerator3")) 300.0))

(event `ShortRangeAttack`
  (params (AttackTarget :type "Actor Object Reference"))
  ;[1 1 1] Attacks
  (`/Game/Attacks/BPC_Attacks.PrimaryMeleeAttack` (`self.BPC_Attacks`) (make `/Game/Attacks/S_AttackInfo` AttackTarget "/Game/Characters/Toilets/Toilet1/Animations/AM_BiteNeq.AM_BiteNeq" (make `/Game/DamageSystem/S_DamageInfo` 10.0 "NewEnumerator1" "NewEnumerator0" false true true)) 20.0 200.0))

(event `LongRangeAttack`
  (params (AttackTarget :type "Actor Object Reference"))
  ;[1 1 1] Attacks
  (`/Game/Attacks/BPC_Attacks.LongRangeMeleeAttack` (`self.BPC_Attacks`) (make `/Game/Attacks/S_AttackInfo` AttackTarget "/Game/Characters/Toilets/Toilet1/Animations/AM_Bite.AM_Bite" (make `/Game/DamageSystem/S_DamageInfo` 10.0 "NewEnumerator1" "NewEnumerator0" false true true))))

(event `SpinningAttack`
  (params (AttackTarget :type "Actor Object Reference"))
  ;[1 1 1] Attacks
  (`/Game/Attacks/BPC_Attacks.SpinningMeleeAttack` (`self.BPC_Attacks`) (make `/Game/Attacks/S_AttackInfo` AttackTarget "/Game/Animations/Melee/Montage_Sword_SpinningAttack.Montage_Sword_SpinningAttack" (make `/Game/DamageSystem/S_DamageInfo` 10.0 "NewEnumerator1" "NewEnumerator0" false true))))

(event `/Game/Enemies/AI/BPI_EnemyAI.EquipWeapon`
  (bind _skibidicalm (`self.SkibidiCalm`))
  ;[1 1 1] Equip/Unequip weapon
  (bind _notifyname (`|PlayMontage` (`self.Mesh`) "/Game/Animations/Melee/Montage_Unsheath_Sword.Montage_Unsheath_Sword")
    (:`then`
      (`AudioComponent.SetVolumeMultiplier` _skibidicalm 0.0))
    (:`OnCompleted`
      (`self.OnWeaponEquipped`)
      (`AudioComponent.SetSound` _skibidicalm "/Game/Audio/skibidi-toilet-attack.skibidi-toilet-attack")
      (`AudioComponent.SetVolumeMultiplier` _skibidicalm 1.0))
    (:`OnNotifyBegin`
      (switch `name` _notifyname
        (:`HoldSword`
          (bind _returnvalue (`|SpawnActorFromClass` "/Game/Weapons/BP_Weapon_Sword.BP_Weapon_Sword_C" (`self.GetTransform`) "Undefined" "MultiplyWithRoot" null null))
          (bind _output_get (set `self.WeaponActor` _returnvalue))
          (`self.K2_AttachToComponent` _output_get (`self.Mesh`) "hand_r_sword_socket" "SnapToTarget" "SnapToTarget" "SnapToTarget" true)
          (set `self.IsWieldingWeapon` true))))))

(event `/Game/Enemies/AI/BPI_EnemyAI.UnequipWeapon`
  (bind _skibidicalm (`self.SkibidiCalm`))
  ;[1 1 1] Equip/Unequip weapon
  (bind _notifyname (`|PlayMontage` (`self.Mesh`) "/Game/Animations/Melee/Montage_Sheath_Sword.Montage_Sheath_Sword")
    (:`then`
      (`AudioComponent.SetVolumeMultiplier` _skibidicalm 0.0))
    (:`OnCompleted`
      (`self.OnWeaponUnequipped`)
      (`AudioComponent.SetSound` _skibidicalm "/Game/Sounds/S_Skibidi_Calm.S_Skibidi_Calm")
      (`AudioComponent.SetVolumeMultiplier` _skibidicalm 1.0))
    (:`OnNotifyBegin`
      (switch `name` _notifyname
        (:`DropSword`
          (`self.K2_DestroyActor` (`self.WeaponActor`))
          (set `self.IsWieldingWeapon` false))))))

(fn `CalculateFutureActorLocation`
  (params (Actor :type "Actor Object Reference") (Time :type "Float (double-precision)" :default 1.0))
  (returns (Location :type "Vector Structure"))
  (return (+ (`self.K2_GetActorLocation` Actor) (* (* (`self.GetVelocity` Actor) (1.0 1.0 0.0)) Time))))

(fn `GetIdealRange`
  (returns (AttackRadius :type "Float (double-precision)") (DefendRadius :type "Float (double-precision)"))
  (return 200.0 400.0))

(fn `IsDead`
  (returns (Dead :type Boolean))
  (return false))

(fn `TakeDamage`
  (params (DamageInfo :type "/Game/DamageSystem/S_DamageInfo Structure") (`Damage Causer` :type "Actor Object Reference"))
  (returns (WasDamaged :type Boolean))
  (return false))

(fn `UserConstructionScript`
  (`parent.UserConstructionScript`)
  (set `self.MeshRotationBeforeSpin` (`SceneComponent.RelativeRotation` (`self.Mesh`))))