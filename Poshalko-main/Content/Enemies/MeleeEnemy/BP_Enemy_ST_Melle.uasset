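; Melee enemy Blueprint, a flushable Skibidi toilet character built on a parent enemy class.
; Attack events pass montage and damage data to BPCAttacks for ground smash, short-range, long-range and spinning attacks.
; Equip and unequip montages use notifies to spawn or destroy a socketed sword, while swapping the SkibidiCalm audio between calm and attack sounds.
; Death mutes that audio and halts movement; flushing plays a sound and emits noise.
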(event `self.ReceiveBeginPlay`
  (`parent.ReceiveBeginPlay`)
  (set `/Game/Systems/DamageSystem/BPC_DamageSystem.IsFlushable` true (`self.BPC_DamageSystem`)))

(event `self.ReceiveTick`
  (params (DeltaSeconds :type "Float (single-precision)"))
  (bind _dead (`/Game/Systems/DamageSystem/BPI_Damagable.IsDead`))
  (if _dead
    (`AudioComponent.SetVolumeMultiplier` (`self.SkibidiCalm`) 0.0)
    (`MovementComponent.StopMovementImmediately` (`self.CharacterMovement`))))

(event `GroundSmashAttack`
  (params (AttackTarget :type "Actor Object Reference"))
  ;[1 1 1] Attacks
  (`/Game/Systems/Attacks/BPC_Attacks.GroundSmash` (`self.BPC_Attacks`) (make `/Game/Systems/Attacks/S_AttackInfo` AttackTarget "/Game/Characters/Toilets/Toilet1/Animations/AM_GroundSmash.AM_GroundSmash" (make `/Game/Systems/DamageSystem/S_DamageInfo` 75.0 "NewEnumerator4" "NewEnumerator3" "NewEnumerator4")) 1000.0))

(event `ShortRangeAttack`
  (params (AttackTarget :type "Actor Object Reference"))
  ;[1 1 1] Attacks
  (`/Game/Systems/Attacks/BPC_Attacks.PrimaryMeleeAttack` (`self.BPC_Attacks`) (make `/Game/Systems/Attacks/S_AttackInfo` AttackTarget "/Game/Characters/Toilets/Toilet1/Animations/AM_BiteNeq.AM_BiteNeq" (make `/Game/Systems/DamageSystem/S_DamageInfo` 50.0 "NewEnumerator1" "NewEnumerator1" "NewEnumerator4" false true true)) 20.0 200.0 0.0))

(event `LongRangeAttack`
  (params (AttackTarget :type "Actor Object Reference"))
  ;[1 1 1] Attacks
  (`/Game/Systems/Attacks/BPC_Attacks.LongRangeMeleeAttack` (`self.BPC_Attacks`) (make `/Game/Systems/Attacks/S_AttackInfo` AttackTarget "/Game/Characters/Toilets/Toilet1/Animations/AM_Bite.AM_Bite" (make `/Game/Systems/DamageSystem/S_DamageInfo` 10.0 "NewEnumerator0" "NewEnumerator1" "NewEnumerator0" false true true))))

(event `SpinningAttack`
  (params (AttackTarget :type "Actor Object Reference"))
  ;[1 1 1] Attacks
  (`/Game/Systems/Attacks/BPC_Attacks.SpinningMeleeAttack` (`self.BPC_Attacks`) (make `/Game/Systems/Attacks/S_AttackInfo` AttackTarget "/Game/Animations/Melee/Montage_Sword_SpinningAttack.Montage_Sword_SpinningAttack" (make `/Game/Systems/DamageSystem/S_DamageInfo` 10.0 "NewEnumerator0" "NewEnumerator1" "NewEnumerator0" false true))))

(event `self.EquipWeapon`
  (bind _skibidicalm (`self.SkibidiCalm`))
  ;[1 1 1] Equip/Unequip weapon
  (bind _notifyname (`|PlayMontage` (`self.Mesh`) "/Game/Animations/Melee/Montage_Unsheath_Sword.Montage_Unsheath_Sword")
    (:`then`
      (`AudioComponent.SetVolumeMultiplier` _skibidicalm 0.0)
      (`AudioComponent.SetSound` _skibidicalm "/Game/Audio/skibidi-toilet-attack.skibidi-toilet-attack"))
    (:`OnCompleted`
      (`self.OnWeaponEquipped`)
      (`AudioComponent.SetVolumeMultiplier` _skibidicalm 1.0 :!label _label))
    (:`OnInterrupted`
      (goto _label))
    (:`OnNotifyBegin`
      (switch `name` _notifyname
        (:`HoldSword`
          (bind _returnvalue (`|SpawnActorFromClass` "/Game/Weapons/BP_Weapon_Sword.BP_Weapon_Sword_C" (`self.GetTransform`) "Undefined" "MultiplyWithRoot" null null))
          (bind _output_get (set `self.WeaponActor` _returnvalue))
          (`self.K2_AttachToComponent` _output_get (`self.Mesh`) "hand_r_sword_socket" "SnapToTarget" "SnapToTarget" "SnapToTarget" true)
          (set `self.IsWieldingWeapon` true))))))

(event `self.UnequipWeapon`
  (bind _skibidicalm (`self.SkibidiCalm`))
  ;[1 1 1] Equip/Unequip weapon
  (bind _notifyname (`|PlayMontage` (`self.Mesh`) "/Game/Animations/Melee/Montage_Sheath_Sword.Montage_Sheath_Sword")
    (:`then`
      (`AudioComponent.SetVolumeMultiplier` _skibidicalm 0.0)
      (`AudioComponent.SetSound` _skibidicalm "/Game/Sounds/S_Skibidi_Calm.S_Skibidi_Calm"))
    (:`OnCompleted`
      (`AudioComponent.SetVolumeMultiplier` _skibidicalm 1.0)
      (`self.OnWeaponUnequipped`))
    (:`OnNotifyBegin`
      (switch `name` _notifyname
        (:`DropSword`
          (`self.K2_DestroyActor` (`self.WeaponActor`))
          (set `self.IsWieldingWeapon` false))))))

(event `Flush_Sound`
  (bind _returnvalue (`self.K2_GetActorLocation`))
  ;[1 1 1] Equip/Unequip weapon
  (`GameplayStatics.PlaySoundAtLocation` "/Game/Sounds/SW_Flushing.SW_Flushing" _returnvalue (struct) 1.0 1.0 0.0 null null null null)
  (`self.MakeNoise` 1.0 null _returnvalue))

(fn `GetGrappleComponent`
  (returns (Component :type "/Game/GrappleComponent/BP_GrappleComponent/GrappleComponent Object Reference"))
  (return (`self.GrappleComponent`)))

(fn `UserConstructionScript`
  (`parent.UserConstructionScript`))