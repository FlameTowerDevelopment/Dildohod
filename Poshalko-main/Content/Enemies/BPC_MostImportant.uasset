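; Enemy-folder component of angle-check helpers for testing where one actor sits relative to another's facing.
; TestConditionAngle combines the target's look-at rotation toward an actor with its negated rotation, then feeds IsRotatorInRange.
; Each axis goes through IsAngleInRange, which handles ±180° wraparound and recurses for optional mirrored ranges.
; Behind only forwards to a Behind call with swapped actors; the rear-cone test in "Behind?" is unused.
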(fn `Behind`
  (params (Kto :type "Actor Object Reference") (Kogo :type "Actor Object Reference") (MaxAngle :type "Float (double-precision)"))
  (returns (Return :type Boolean))
  (return (`self.Behind?` Kogo Kto MaxAngle)))

(fn `Is Angle In Range ?`
  (params (Value :type "Float (double-precision)") (A :type "Float (double-precision)") (B :type "Float (double-precision)") (Mirror :type Boolean))
  (returns (`In Range` :type Boolean))
  (locals (Local_Value :type "Float (double-precision)") (Local_Min :type "Float (double-precision)") (Local_Max :type "Float (double-precision)") (Local_Success :type Boolean))
  (`|ExecutionSequence`
    (:`then_0`
      ;[1 1 1] Set local variables
      (set `local.Local_Value` Value)
      (set `local.Local_Min` A)
      (set `local.Local_Max` B))
    (:`then_1`
      ;[1 1 1] Test a range that passes the 180°/-180° treshold
      (if (< (`local.Local_Min`) (`local.Local_Max`))
        ;[1 1 1] Test a range that does not pass the 180°/-180° treshold
        (set `local.Local_Success` (`KismetMathLibrary.InRange_FloatFloat` (`local.Local_Value`) (`local.Local_Min`) (`local.Local_Max`)))
        (else
          (set `local.Local_Success` (or (`KismetMathLibrary.InRange_FloatFloat` (`local.Local_Value`) (`local.Local_Min`) 180.0) (`KismetMathLibrary.InRange_FloatFloat` (`local.Local_Value`) -180.0 (`local.Local_Max`)))))))
    (:`then_2`
      ;[1 1 1] Test mirrored range
      (if Mirror
        (bind _output_get (set `local.Local_Success` (or (`self.Is Angle In Range ?` (`local.Local_Value`) (* (`local.Local_Max`) -1.0) (* (`local.Local_Min`) -1.0)) (`local.Local_Success`))))
        (return _output_get)
        (else
          (return (`local.Local_Success`)))))))

(fn `Is rotator in range`
  (params (`Rotator to check` :type "Rotator Structure") (`Range A` :type "Rotator Structure") (`Range B` :type "Rotator Structure") (`Mirror X` :type Boolean) (`Mirror Y` :type Boolean) (`Mirror Z` :type Boolean))
  (returns (`InRange?` :type Boolean))
  (locals (Local_MirrorX :type Boolean) (Local_MirrorY :type Boolean) (Local_MirrorZ :type Boolean) (Local_rangeA :type "Rotator Structure") (Local_rangeB :type "Rotator Structure") (Local_RotatorToCheck :type "Rotator Structure"))
  ;[1 1 1] Calculate if the values is in range A to B of the provided rotator for each axis
  (`|ExecutionSequence`
    (:`then_0`
      ;[0.4534 1 0.4479] Set local variables
      (set `local.Local_MirrorX` `Mirror X`)
      (set `local.Local_MirrorY` `Mirror Y`)
      (set `local.Local_MirrorZ` `Mirror Z`)
      (set `local.Local_rangeA` `Range A`)
      (set `local.Local_rangeB` `Range B`)
      (set `local.Local_RotatorToCheck` `Rotator to check`))
    (:`then_1`
      (return (and (`self.Is Angle In Range ?` (.roll (`local.Local_RotatorToCheck`)) (.roll (`local.Local_rangeA`)) (.roll (`local.Local_rangeB`)) (`local.Local_MirrorX`)) (`self.Is Angle In Range ?` (.pitch (`local.Local_RotatorToCheck`)) (.pitch (`local.Local_rangeA`)) (.pitch (`local.Local_rangeB`)) (`local.Local_MirrorY`)) (`self.Is Angle In Range ?` (.yaw (`local.Local_RotatorToCheck`)) (.yaw (`local.Local_rangeA`)) (.yaw (`local.Local_rangeB`)) (`local.Local_MirrorZ`)))))))

(fn `TestConditionAngle`
  (params (ActorRef :type "Actor Object Reference") (Target :type "Actor Object Reference") (RangeA :type "Rotator Structure") (RangeB :type "Rotator Structure") (`Mirror X` :type Boolean) (`Mirror Y` :type Boolean) (`Mirror Z` :type Boolean))
  (returns (`Condition Fulfilled` :type Boolean))
  (`|ExecutionSequence`
    (:`then_0`
      (bind _inrange_ (`self.Is rotator in range` (`KismetMathLibrary.ComposeRotators` (`KismetMathLibrary.FindLookAtRotation` (`Actor.K2_GetActorLocation` Target) (`Actor.K2_GetActorLocation` (select `bool` (`KismetSystemLibrary.IsValid` ActorRef) :`false` ActorRef :`true` ActorRef))) (* (`Actor.K2_GetActorRotation` Target) -1.0)) RangeA RangeB `Mirror X` `Mirror Y` `Mirror Z`))
      (return _inrange_))))