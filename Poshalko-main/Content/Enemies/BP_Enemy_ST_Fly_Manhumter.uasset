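; Flying saw-blade "Manhunter" enemy that rams its target, then crashes and explodes once damaged.
; On spawn it sphere-traces for a pawn; each tick it spins rotor and saw, deals close-range damage, faces the target and randomly lunges via impulses.
; BPCDamageSystem damage responses switch it to physics-driven falling, where a hit or further damage triggers explosion and BPCAttacks area damage.
; Most other combat-interface functions are stubs.
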(event `self.ReceiveBeginPlay`
  (`self.On spawned`))

(event `self.ReceiveTick`
  (params (DeltaSeconds :type "Float (single-precision)"))
  (bind _saw (`self.Saw`))
  (bind (_relativerotation_roll _relativerotation_pitch _relativerotation_yaw) (`KismetMathLibrary.BreakRotator` (`SceneComponent.RelativeRotation` _saw)))
  (if (`self.IsFalling`)
    (`PrimitiveComponent.SetSimulatePhysics` (`self.CapsuleComponent`) true)
    (`CharacterMovementComponent.SetMovementMode` (`self.CharacterMovement`) "MOVE_Walking" 0)
    (else
      (`SceneComponent.K2_AddRelativeRotation` (`self.HeliScrew`) (struct :`Yaw` 50.0) false false)
      (`SceneComponent.K2_SetRelativeRotation` _saw (`KismetMathLibrary.MakeRotator` _relativerotation_roll _relativerotation_pitch (+ _relativerotation_yaw 10.0)) false false)
      (`/Game/Systems/Attacks/BPC_Attacks.SphereTraceDamage` (`self.BPC_Attacks`) (make `/Game/Systems/DamageSystem/S_DamageInfo` 1.0) 100.0 0.0)
      (`self.K2_SetActorRotation` (`KismetMathLibrary.FindLookAtRotation` (`self.K2_GetActorLocation`) (`self.K2_GetActorLocation` (`self.AttackTarget`))))
      (if (< (`KismetMathLibrary.RandomFloat`) 0.01)
        (`CharacterMovementComponent.AddImpulse` (`self.CharacterMovement`) (* (`KismetMathLibrary.GetForwardVector` (`self.K2_GetActorRotation`)) 500.0) true)
        (`GameplayStatics.PlaySoundAtLocation` "/Game/Audio/manhack/blade_loop1.blade_loop1" (`self.K2_GetActorLocation`) (struct) 1.0 1.0 0.0 null null null null)))))

(event `self.ReceiveHit`
  (params (MyComp :type "PrimitiveComponent Object Reference") (Other :type "Actor Object Reference") (OtherComp :type "PrimitiveComponent Object Reference") (bSelfMoved :type Boolean) (HitLocation :type "Vector Structure") (HitNormal :type "Vector Structure") (NormalImpulse :type "Vector Structure") (Hit :type "HitResult Structure (by ref)"))
  (bind _returnvalue (`self.K2_GetActorLocation`))
  (if (`self.IsFalling`)
    (`PrimitiveComponent.SetCollisionEnabled` (`self.CapsuleComponent`) "NoCollision")
    (`PrimitiveComponent.SetCollisionEnabled` (`self.CapsuleComponent`) "NoCollision")
    (`SceneComponent.SetVisibility` (`self.CapsuleComponent`) false true)
    (`GameplayStatics.SpawnEmitterAtLocation` "/Game/StarterContent/Particles/P_Explosion.P_Explosion" _returnvalue (struct) (3.0 3.0 3.0))
    (`GameplayStatics.PlaySoundAtLocation` "/Game/StarterContent/Audio/Explosion01.Explosion01" _returnvalue (struct) 1.0 1.0 0.0 null null null null)
    (`AudioComponent.SetVolumeMultiplier` (`self.engine_loop1`) 0.0)
    (`AudioComponent.SetVolumeMultiplier` (`self.skibidi-toilet-attack`) 0.0)
    (`self.Die`)))

(event `Die`
  (set `/Game/Systems/DamageSystem/BPC_DamageSystem.IsDead` true (`self.BPC_DamageSystem`))
  (`/Game/Systems/Attacks/BPC_Attacks.SphereTraceDamage` (`self.BPC_Attacks`) (make `/Game/Systems/DamageSystem/S_DamageInfo` 30.0 "NewEnumerator1" "NewEnumerator3" "NewEnumerator4" true true true) 300.0 0.0))

(event `DamageResponce`
  (params (DamageResponse :type "/Game/Systems/DamageSystem/E_DamageResponse Enum" :default "NewEnumerator0") (DamageCauser :type "Actor Object Reference") (ImpactType :type "/Game/Systems/DamageSystem/E_DamageImpactType Enum" :default "NewEnumerator0"))
  (bind _returnvalue (`self.K2_GetActorLocation`))
  (if (`self.IsFalling`)
    (`PrimitiveComponent.SetCollisionEnabled` (`self.CapsuleComponent`) "NoCollision")
    (`PrimitiveComponent.SetCollisionEnabled` (`self.CapsuleComponent`) "NoCollision")
    (`SceneComponent.SetVisibility` (`self.CapsuleComponent`) false true)
    (`GameplayStatics.SpawnEmitterAtLocation` "/Game/StarterContent/Particles/P_Explosion.P_Explosion" _returnvalue (struct) (3.0 3.0 3.0))
    (`GameplayStatics.PlaySoundAtLocation` "/Game/StarterContent/Audio/Explosion01.Explosion01" _returnvalue (struct) 1.0 1.0 0.0 null null null null)
    (`AudioComponent.SetVolumeMultiplier` (`self.skibidi-toilet-attack`) 0.0)
    (`self.Die`)
    (else
      (`CharacterMovementComponent.SetMovementMode` (`self.CharacterMovement`) "MOVE_Walking" 0)
      (`GameplayStatics.PlaySoundAtLocation` "/Game/Sounds/Skibidi_Scream.Skibidi_Scream" (`self.K2_GetActorLocation`) (struct) 1.0 1.0 0.0 null null null null)
      (`KismetSystemLibrary.Delay` 0.1)
      (set `self.IsFalling` true)
      (`AudioComponent.SetVolumeMultiplier` (`self.engine_loop1`) 0.0))))

(event `/Game/Systems/DamageSystem/BPI_Damagable.ReturnAttackToken`
  (params (Amount :type Integer))
  (`/Game/Systems/DamageSystem/BPC_DamageSystem.ReturnAttackToken` (`self.BPC_DamageSystem`) Amount))

(event `/Game/Systems/DamageSystem/BPI_Damagable.SetIsInvincible`
  (params (Value :type Boolean))
  (set `/Game/Systems/DamageSystem/BPC_DamageSystem.IsInvincible` Value (`self.BPC_DamageSystem`)))

(event `/Game/Enemies/AI/BPI_EnemyAI.StoreAttackTokens`
  (params (AttackTarget :type "Actor Object Reference") (Amount :type Integer)))

(event `On spawned`
  (bind _returnvalue (`self.K2_GetActorLocation`))
  (bind _bpc_damagesystem (`self.BPC_DamageSystem`))
  (bind _bpc_damagesystem_2 (`self.BPC_DamageSystem`))
  (set `/Game/Systems/DamageSystem/BPC_DamageSystem.Health` 100.0 _bpc_damagesystem_2)
  (set `/Game/Systems/DamageSystem/BPC_DamageSystem.AttackTokensCount` 3 _bpc_damagesystem_2)
  (`/Engine/EditorBlueprintResources/StandardMacros.IsValid` (`self.AttackTarget`)
    (:`Is Valid`
      _)
    (:`Is Not Valid`
      (bind _outhit (`KismetSystemLibrary.SphereTraceSingleForObjects` :`Start` _returnvalue :`End` _returnvalue :`Radius` 1000.0 :`ObjectTypes` (`|MakeArray` "ObjectTypeQuery3" :!type "EObjectTypeQuery Enum") :`DrawDebugType` "ForDuration"))
      (set `self.AttackTarget` (`.HitActor` (`GameplayStatics.BreakHitResult` _outhit)))))
  (`CharacterMovementComponent.AddImpulse` (`self.CharacterMovement`) (* (`KismetMathLibrary.GetForwardVector` (`self.K2_GetActorRotation`)) 500.0) true)
  (add `/Game/Systems/DamageSystem/BPC_DamageSystem.OnDeath` _bpc_damagesystem (`|CreateDelegate` :!event `Die`))
  (add `/Game/Systems/DamageSystem/BPC_DamageSystem.OnDamageResponse` _bpc_damagesystem (`|CreateDelegate` :!event `DamageResponce`))
  (set `self.IsFalling` false))

(fn `AttackStart`
  (params (AttackTarget :type "Actor Object Reference") (TokensNeeded :type Integer))
  (returns (Success :type Boolean))
  (return false))

(fn `GetCurrentHealth`
  (returns (Health :type "Float (double-precision)"))
  (return 0.0))

(fn `GetIdealRange`
  (returns (AttackRadius :type "Float (double-precision)") (DefendRadius :type "Float (double-precision)"))
  (return 0.0 0.0))

(fn `GetMaxHealth`
  (returns (MaxHealth :type "Float (double-precision)"))
  (return 0.0))

(fn `GetPatrolRoute`
  (returns (PatrolRoute :type "/Game/Enemies/AI/BP_PatrolRoute Object Reference"))
  (return null))

(fn `GetTeamNumber`
  (returns (TeamNumber :type Integer))
  (return (`self.TeamNumber`)))

(fn `Heal`
  (params (Amount :type "Float (double-precision)"))
  (returns (NewHealth :type "Float (double-precision)"))
  (return 0.0))

(fn `IsAttacking`
  (returns (Attacking :type Boolean))
  (return false))

(fn `IsDead`
  (returns (Dead :type Boolean))
  (return (`/Game/Systems/DamageSystem/BPC_DamageSystem.IsDead` (`self.BPC_DamageSystem`))))

(fn `ReserveAttackToken`
  (params (Amount :type Integer))
  (returns (Success :type Boolean))
  (bind _success (`/Game/Systems/DamageSystem/BPC_DamageSystem.ReserveAttackToken` (`self.BPC_DamageSystem`) Amount))
  (return _success))

(fn `SetMovementSpeed`
  (params (Speed :type "/Game/Enemies/AI/Enums/E_MovementSpeed Enum" :default "NewEnumerator0"))
  (returns (SpeedValue :type "Float (double-precision)"))
  (return 0.0))

(fn `TakeDamage`
  (params (DamageInfo :type "/Game/Systems/DamageSystem/S_DamageInfo Structure") (`Damage Causer` :type "Actor Object Reference"))
  (returns (WasDamaged :type Boolean))
  (if (not (`.CanBeBlocked_13_824961894D871A8CAC9433AE0314CCBE` (break `/Game/Systems/DamageSystem/S_DamageInfo` DamageInfo)))
    (bind _wasdamaged (`/Game/Systems/DamageSystem/BPC_DamageSystem.TakeDamage` (`self.BPC_DamageSystem`) DamageInfo `Damage Causer`))
    (return _wasdamaged)))

(fn `UserConstructionScript`)